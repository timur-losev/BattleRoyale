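; Base Blueprint for items, holding a type, name and amount.
; BeginPlay caches references to the player's MyCharacter and MyPlayerController.
; Init sets the type and name, and UpdateAmount adds to, subtracts from or directly sets the amount based on its Add and Reduce flags.
; GetWeight is a placeholder that returns zero.
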(event `self.ReceiveBeginPlay`
  ;[1 1 1] Init objects
  (bind _asmy_character (cast `/Game/Blueprint/Character/MyCharacter` (`GameplayStatics.GetPlayerCharacter` 0)))
  (set `self.CharacterRef` _asmy_character)
  (bind _asmy_player_controller (cast `/Game/Blueprint/Gameplay/MyPlayerController` (`GameplayStatics.GetPlayerController` 0)))
  (set `self.ControllerRef` _asmy_player_controller))

(fn `GetWeight`
  (returns (Weight :type Integer))
  (return 0))

(fn `Init`
  (params (ItemType :type "/Game/Blueprint/Datas/Enum/E_ItemType Enum" :default "NewEnumerator0") (Name :type Text))
  (set `self.ItemType` ItemType)
  (set `self.Name` Name))

(fn `UpdateAmount`
  (params (`Add?` :type Boolean) (`Reduce?` :type Boolean) (Amount :type Integer))
  (if `Add?`
    (set `self.Amount` (+ Amount (`self.Amount`)))
    (elif `Reduce?`
      (set `self.Amount` (- (`self.Amount`) Amount))
      (else
        (set `self.Amount` Amount)))))

(fn `UserConstructionScript`)