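; Player controller that drives MyCharacter's movement and mouse look, with a hold-Left-Alt free look.
; Movement follows control yaw and ramps MaxWalkSpeed up from current velocity toward WalkSpeed.
; Tick aligns the character to control yaw and prints its speed; holding Alt suspends alignment and moves along the saved rotation.
; On release, a timeline lerps the control rotation back along the shortest path before normal steering resumes.
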(event `self.ReceiveBeginPlay`
  (`WidgetBlueprintLibrary.SetInputMode_GameOnly` self)
  (set `self.MyCharacterRef` (cast `/Game/Blueprint/Character/MyCharacter` (`GameplayStatics.GetPlayerCharacter` 0) :!pure true)))

(event `InputAxis|MoveForward`
  (params (AxisValue :type "Float (single-precision)"))
  (`self.MovingOnTheGround` true AxisValue (`self.GetControllerRotation`)))

(event `InputAxis|Turn`
  (params (AxisValue :type "Float (single-precision)"))
  (`/Game/Blueprint/Character/MyCharacter.MouseTurn` (`self.MyCharacterRef`) AxisValue))

(event `InputAxis|MoveRight`
  (params (AxisValue :type "Float (single-precision)"))
  (`self.MovingOnTheGround` false AxisValue (`self.GetControllerRotation`)))

(event `InputAxis|LookUp`
  (params (AxisValue :type "Float (single-precision)"))
  (`/Game/Blueprint/Character/MyCharacter.MouseLookUp` (`self.MyCharacterRef`) (* AxisValue -1.0)))

(event `self.ReceiveTick`
  (params (DeltaSeconds :type "Float (single-precision)"))
  (bind (_returnvalue_roll _returnvalue_pitch _returnvalue_yaw) (`KismetMathLibrary.BreakRotator` (`self.GetControlRotation`)))
  (`|ExecutionSequence`
    (:`then_0`
      (if (not (`self.IsAltPressed?`))
        (`self.K2_SetActorRotation` (`self.MyCharacterRef`) (`KismetMathLibrary.MakeRotator` 0.0 0.0 _returnvalue_yaw) false)))
    (:`then_1`
      (`KismetSystemLibrary.PrintString` (`KismetStringLibrary.Conv_DoubleToString` (`KismetMathLibrary.VSize` (`MovementComponent.Velocity` (`Pawn.GetMovementComponent` (`self.MyCharacterRef`)))))))))

(event `InputAction|LeftAlt`
  (params (Key :type "Key Structure"))
  (bind _returnvalue (`SpringArmComponent.GetTargetRotation` (`/Game/Blueprint/Character/MyCharacter.SpringArm` (`self.MyCharacterRef`))))
  (:`Pressed`
    (set `self.IsAltPressed?` true)
    (set `self.AltPressedRotation` _returnvalue))
  (:`Released`
    (set `self.AltReleasedRotation` _returnvalue)
    (bind (_direction _percentage) (`Timeline|TL_CameraRestore` :!via `PlayFromStart`)
      (:`Update`
        (`self.SetControlRotation` (`KismetMathLibrary.RLerp` (`self.AltReleasedRotation`) (`self.AltPressedRotation`) _percentage true)))
      (:`Finished`
        (set `self.IsAltPressed?` false)))))

(fn `GetControllerRotation`
  (returns (Rotation :type "Rotator Structure"))
  (locals (ReturnRotation :type "Rotator Structure"))
  (if (`self.IsAltPressed?`)
    (set `local.ReturnRotation` (`self.AltPressedRotation`))
    (else
      (set `local.ReturnRotation` (`self.GetControlRotation`))))
  (return (`local.ReturnRotation`)))

(fn `MovingOnTheGround`
  (params (Forward :type Boolean) (AxisValue :type "Float (double-precision)") (ControllerRotation :type "Rotator Structure"))
  (bind _walkspeed (`self.WalkSpeed`))
  (bind _mycharacterref (`self.MyCharacterRef`))
  (bind _returnvalue (`KismetMathLibrary.MakeRotator` 0.0 0.0 (.yaw ControllerRotation)))
  (bind _charactermovement (`Character.CharacterMovement` (`self.MyCharacterRef`)))
  (bind _returnvalue_2 (+ (`KismetMathLibrary.VSize` (`MovementComponent.Velocity` (`Character.CharacterMovement` (`self.MyCharacterRef`)))) 5.0))
  (if (<= _returnvalue_2 _walkspeed)
    (set `CharacterMovementComponent.MaxWalkSpeed` _returnvalue_2 _charactermovement)
    (else
      (set `CharacterMovementComponent.MaxWalkSpeed` _walkspeed _charactermovement)))
  (if Forward
    (`Pawn.AddMovementInput` _mycharacterref (`KismetMathLibrary.GetForwardVector` _returnvalue) AxisValue false)
    (else
      (`Pawn.AddMovementInput` _mycharacterref (`KismetMathLibrary.GetRightVector` _returnvalue) AxisValue false))))

(fn `UserConstructionScript`)